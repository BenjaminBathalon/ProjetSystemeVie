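; AC_Hilt is a health component that handles damage, healing and reset for its owner.
; Damage and heal events are ignored while dead; reset clears the dead flag and restores maximum health.
; All three route through UpdateHelthAndNotify, which clamps health, fires OnHealChange, then sets the dead state and fires OnDeath at zero.
; Debug strings print on damage and on every update.
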(event `/Game/Game/Blueprints/Interfaces/BPI_Damageable.TakeDommage`
  (params (DommageAconte :type "Float (double-precision)"))
  (if (not (`self.IsDead`))
    (`self.UpdateHelthAndNotify` (- (`self.CurrentHelth`) DommageAconte))
    (`KismetSystemLibrary.PrintString` "Damage")))

(event `/Game/Game/Blueprints/Interfaces/BPI_Damageable.GainHeal`
  (params (HiltAmount :type "Float (double-precision)"))
  (if (not (`self.IsDead`))
    (`self.UpdateHelthAndNotify` (+ (`self.CurrentHelth`) HiltAmount))))

(event `/Game/Game/Blueprints/Interfaces/BPI_Damageable.ResetHilt`
  (set `self.IsDead` false)
  (`self.UpdateHelthAndNotify` (`self.MaxHelth`)))

(fn `UpdateHelthAndNotify`
  (params (NewHelthValue :type "Float (double-precision)"))
  (bind _maxhelth (`self.MaxHelth`))
  (bind _output_get (set `self.CurrentHelth` (`KismetMathLibrary.FClamp` NewHelthValue 0.0 _maxhelth)))
  (`self.OnHealChange` _output_get _maxhelth)
  (`KismetSystemLibrary.PrintString` "Update")
  (if (<= (`self.CurrentHelth`) 0.0)
    (set `self.IsDead` true)
    (`self.OnDeath`)
    (else
      (set `self.IsDead` false))))