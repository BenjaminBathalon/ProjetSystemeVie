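; BP_PlayerState keeps the player's health in BP_GameInstance and triggers a respawn on death.
; On BeginPlay it either loads current and max health from the game instance into the AC_Hilt health component or, on first initialization, resets the component and sets a flag.
; The component's health-change event writes both values back to the game instance, and its death event calls StartRespawn on BP_ThirdPersonGameMode for player controller 0.
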(event `self.ReceiveBeginPlay`
  (bind _asbp_game_instance (cast `/Game/Game/BP_GameInstance` (`GameplayStatics.GetGameInstance`)))
  (bind _output_get (set `self.REF Game Instance` _asbp_game_instance))
  (if (`/Game/Game/BP_GameInstance.HealthInitialize_GI` _output_get)
    (`self.LoadHealthFromGI`)
    (else
      (`/Game/Game/Blueprints/Components/AC_Hilt.ResetHilt` (`self.AC_Hilt`))
      (set `/Game/Game/BP_GameInstance.HealthInitialize_GI` true (`self.REF Game Instance`)))))

(event `self.AC_Hilt.OnHealChange`
  (params (CurrentHelth :type "Float (double-precision)") (MaxHelth :type "Float (double-precision)"))
  (`self.SaveCurrentHealth` CurrentHelth)
  (`self.SaveMaxHealth` MaxHelth))

(event `self.AC_Hilt.OnDeath`
  (bind _asbp_third_person_game_mode (cast `/Game/Game/Blueprints/GameModes/BP_ThirdPersonGameMode` (`GameplayStatics.GetGameMode`)))
  (`/Game/Game/Blueprints/GameModes/BP_ThirdPersonGameMode.StartRespawn` _asbp_third_person_game_mode (`GameplayStatics.GetPlayerController` 0)))

(fn `LoadHealthFromGI`
  (bind _ref_game_instance (`self.REF Game Instance`))
  (bind _ac_hilt (`self.AC_Hilt`))
  (bind _output_get (set `/Game/Game/Blueprints/Components/AC_Hilt.CurrentHelth` (`/Game/Game/BP_GameInstance.CurrentHealth_GI` _ref_game_instance) _ac_hilt))
  (bind _output_get_2 (set `/Game/Game/Blueprints/Components/AC_Hilt.MaxHelth` (`/Game/Game/BP_GameInstance.MaxHealth_GI` _ref_game_instance) _ac_hilt))
  (`/Game/Game/Blueprints/Components/AC_Hilt.OnHealChange` (`self.AC_Hilt`) _output_get _output_get_2))

(fn `SaveCurrentHealth`
  (params (NewHealth :type "Float (double-precision)"))
  (set `/Game/Game/BP_GameInstance.CurrentHealth_GI` NewHealth (`self.REF Game Instance`)))

(fn `SaveMaxHealth`
  (params (NewMaxHealth :type "Float (double-precision)"))
  (set `/Game/Game/BP_GameInstance.MaxHealth_GI` NewMaxHealth (`self.REF Game Instance`)))

(fn `UserConstructionScript`)